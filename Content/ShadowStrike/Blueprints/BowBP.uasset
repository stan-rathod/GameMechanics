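; Bow weapon actor that shows itself only while its parent actor aims and supplies values for adjusting the bowstring.
; AdjustBowDraw sets visibility and plays a timeline into BowAlpha, resetting it and HandLocation when aiming stops.
; While aiming, Tick pulls the hand location from the parent through a message call, and getters expose both values.
; ToggleVFX swaps bow and arrow materials and retargets the fire particles' surface actor for wraith mode.
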(event Custom|Adjust%20Bow%20Draw
  (params (isAiming? :type Boolean))
  ;[1 1 1] Update bow alpha value to adjust the bow string when aiming
  (bind _output_get (Variables|Default|SetisAiming? isAiming?))
  (CallFunction|ToggleVisibility (not _output_get))
  (if _output_get
    (bind _alpha (Timeline|DrawAlpha Play)
      (:Update
        (Variables|Default|SetBowAlpha _alpha)))
    (else
      (Variables|Default|SetBowAlpha 0.0)
      (Variables|Default|SetHandLocation "0, 0, 0"))))

(event EventBeginPlay
  ;[0.2984 0.5231 1] Store ref of anim bp of bow at start (if there is a anim bp for BOW)
)

(event Collision|EventActorBeginOverlap
  (params (OtherActor :type Actor%20Object%20Reference)))

(event EventTick
  (params (DeltaSeconds :type Float%20%28single-precision%29))
  ;[0 0.3836 1] Update owner hand location when aiming
  (if (Variables|Default|GetisAiming?)
    (CallFunction|SetOwnerHandLocation)))

(event EventToggleVisibility
  (params (Hide? :type Boolean))
  ;[1 1 1] Toggle bow visibility
  (if Hide?
    (Rendering|SetVisibility (Variables|Default|GetDefaultSceneRoot) false true)
    (else
      (Rendering|SetVisibility (Variables|Default|GetDefaultSceneRoot) true true))))

(fn ConstructionScript)

(fn GetBowAlpha
  (return (Variables|Default|GetBowAlpha)))

(fn SetOwnerHandLocation
  (bind _location (Class|BPICharacter|GetBowHandLocation(Message) (Actor|GetParentActor)))
  (Variables|Default|SetHandLocation _location))

(fn GetHandLocation
  (return (Variables|Default|GetHandLocation)))

(fn ToggleVFX
  (params (Show? :type Boolean))
  (bind _arrow (Variables|Default|GetArrow))
  (bind _arrow_2 (Variables|Default|GetArrow))
  (if Show?
    ;[0 0.8071 1] Update the material of the wepaon when warith mode and toggle the fire particle effect
    (Effects|Components|ParticleSystem|SetActorParameter (Variables|Default|GetParticleSystem) "VertSurfaceActor" self)
    (Rendering|Material|SetMaterial (Variables|Default|GetSkeletalMesh) 0 0)
    (Utilities|FlowControl|Sequence
      (:then_0
        (Rendering|Material|SetMaterial _arrow_2 0 0))
      (:then_1
        (Rendering|Material|SetMaterial _arrow_2 1 0))
      (:then_2
        (Rendering|Material|SetMaterial _arrow_2 2 0)))
    (else
      (Effects|Components|ParticleSystem|SetActorParameter (Variables|Default|GetParticleSystem) "VertSurfaceActor" 0)
      (Rendering|Material|SetMaterial (Variables|Default|GetSkeletalMesh) 0 0)
      (Utilities|FlowControl|Sequence
        (:then_0
          (Rendering|Material|SetMaterial _arrow 0 0))
        (:then_1
          (Rendering|Material|SetMaterial _arrow 1 0))
        (:then_2
          (Rendering|Material|SetMaterial _arrow 2 0))))))