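; Animation notify state for Shadow Strike that drives time dilation and an optional chain-attack window on the mesh owner through interface messages.
; Begin sends the configured time dilation to the owner, and end restores it to normal.
; With ActivateChain set, each tick asks the owner to trace enemies for a chain attack and end signals chain timer expiry.
; Otherwise, end tells the owner to enable Wraith Flash.
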(fn ReceivedNotifyBegin
  (params (MeshComp :type Skeletal%20Mesh%20Component%20Object%20Reference) (Animation :type Anim%20Sequence%20Base%20Object%20Reference) (TotalDuration :type Float%20%28single-precision%29))
  (bind _returnvalue (Components|GetOwner MeshComp))
  (Utilities|IsValid _returnvalue
    (:Is%20Valid
      (Class|BPICharacter|UpdateGlobalTimeDialation(Message) _returnvalue (Variables|Default|GetTimeDialation))
      (return true))))

(fn ReceivedNotifyEnd
  (params (MeshComp :type Skeletal%20Mesh%20Component%20Object%20Reference) (Animation :type Anim%20Sequence%20Base%20Object%20Reference))
  (bind _returnvalue (Components|GetOwner MeshComp))
  (Utilities|IsValid _returnvalue
    (:Is%20Valid
      (Class|BPICharacter|UpdateGlobalTimeDialation(Message) _returnvalue 1.0)
      (if (Variables|Default|GetActivateChain?)
        (Class|BPICharacter|OnChainTimerExpired(Message) _returnvalue)
        (return true)
        (else
          (Class|BPICharacter|EnableWraithFlash(Message) _returnvalue)
          (return true))))))

(fn ReceivedNotifyTick
  (params (MeshComp :type Skeletal%20Mesh%20Component%20Object%20Reference) (Animation :type Anim%20Sequence%20Base%20Object%20Reference) (FrameDeltaTime :type Float%20%28single-precision%29))
  (bind _returnvalue (Components|GetOwner MeshComp))
  (if (Variables|Default|GetActivateChain?)
    (Utilities|IsValid _returnvalue
      (:Is%20Valid
        (Class|BPICharacter|TraceEnemiesforChainAttack(Message) _returnvalue)
        (return false)))))